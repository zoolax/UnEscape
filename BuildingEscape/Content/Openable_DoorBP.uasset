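; Openable door actor that swings open and closed in response to open and close requests from its OpemDoor member.
; It caches its initial rotation on BeginPlay, and the DoorSwing timeline plays forward to open and in reverse to close.
; Each timeline update combines an animated yaw angle with that initial rotation.
; A timeline event track plays the Magic_02 sound at the door's location.
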(event OnOpenRequest(OpemDoor)
  (bind _open_angle (Timeline|Door%20Swing Play)
    (:Update
      (Transformation|SetActorRotation (Math|Rotator|CombineRotators (Math|Rotator|MakeRotator 0.0 0.0 _open_angle) (Variables|Default|GetInitialRotation))))
    (:SoundE
      (Audio|PlaySoundatLocation "/Game/magic_02.magic_02" (Transformation|GetActorLocation)))))

(event OnCloseRequest(OpemDoor)
  (bind _open_angle (Timeline|Door%20Swing Reverse)
    (:Update
      (Transformation|SetActorRotation (Math|Rotator|CombineRotators (Math|Rotator|MakeRotator 0.0 0.0 _open_angle) (Variables|Default|GetInitialRotation))))
    (:SoundE
      (Audio|PlaySoundatLocation "/Game/magic_02.magic_02" (Transformation|GetActorLocation)))))

(event EventBeginPlay
  (Variables|Default|SetInitialRotation (Transformation|GetActorRotation)))

(fn ConstructionScript)